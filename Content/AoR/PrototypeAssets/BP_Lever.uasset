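; BP_Lever is a prototype interactable lever that switches a linked gate.
; Interact plays or reverses the LeverAnim timeline depending on OnOff, rolling the LeverHandle through its relative rotation.
; When the timeline finishes, it flips OnOff and passes the new state to TargetGate through SwitchMessage, so the gate responds only after the handle stops moving.
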(event EventInteract
  (if (Variables|Default|GetOn/Off)
    (bind _leverrotation (Timeline|LeverAnim Play)
      (:Update
        (Transformation|SetRelativeRotation (Variables|Default|GetLeverHandle) (Math|Rotator|MakeRotator _leverrotation 0.0 0.0) false false))
      (:Finished
        (bind _output_get (Variables|Default|SetOn/Off (not (Variables|Default|GetOn/Off))))
        (Class|BPIGateControl|Switch(Message) (Variables|Default|GetTargetGate) _output_get)))
    (else
      (Timeline|LeverAnim Reverse))))

(fn ConstructionScript
  (|CallParentFunction))