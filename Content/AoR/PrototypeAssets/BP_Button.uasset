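; BP_Button is a prototype interactable button that switches a linked TargetGate on for a short time.
; Interact plays a timeline that moves the button along its local Y axis, then sends SwitchMessage(true) to the gate when finished.
; After a short delay, a second timeline animates the button again and sends SwitchMessage(false) on every update rather than once at the end.
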(event EventInteract
  (bind _buttonposition (Timeline|ButtonAnim1 Play)
    (:Update
      (Transformation|SetRelativeLocation (Variables|Default|GetButton) (Math|Vector|MakeVector 0.0 _buttonposition 5.0) false false))
    (:Finished
      (Class|BPIGateControl|Switch(Message) (Variables|Default|GetTargetGate) true)
      (Utilities|FlowControl|Delay 3.0)
      (bind _buttonposition_2 (Timeline|ButtonAnin2 Play)
        (:Update
          (Transformation|SetRelativeLocation (Variables|Default|GetButton) (Math|Vector|MakeVector 0.0 _buttonposition_2 5.0) false false)
          (Class|BPIGateControl|Switch(Message) (Variables|Default|GetTargetGate) false))))))

(fn ConstructionScript
  (|CallParentFunction))